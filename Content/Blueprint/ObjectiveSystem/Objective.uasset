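; Objective Blueprint for a mission system, typed as Kill, Destruction or Targets.
; Init only handles Targets, registering itself as owner on the TargetMananger, then storing a target count and building "Remaining" text.
; IsObjectiveComplete unconditionally sets Complete and fires the ObjectiveComplete dispatcher.
; The active-target lookup in TargetsLength and a construction-script debug line are left unwired.
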(fn `Init`
  (params (Type :type "/Game/Blueprint/ObjectiveSystem/ObjectiveType Enum" :default "NewEnumerator0"))
  (switch `/Game/Blueprint/ObjectiveSystem/ObjectiveType` Type
    (:`NewEnumerator0`
      (return))
    (:`NewEnumerator1`
      (return))
    (:`NewEnumerator2`
      (bind _compete (`/Game/Blueprint/Managers/TargetManager.SetOwningObjective` (`self.TargetMananger`) self))
      (if _compete
        (set `self.TextNum` (`self.TargetsLength`))
        (`self.UpdateText`)))))

(fn `IsObjectiveComplete`
  (bind _output_get (set `self.Complete` true))
  (`self.ObjectiveComplete` self _output_get))

(fn `UpdateText`
  (returns (Text :type Text))
  (return (`KismetTextLibrary.Conv_StringToText` (`KismetStringLibrary.Concat_StrStr` (`KismetTextLibrary.Conv_TextToString` (`self.Text`)) " Remaining : " (`KismetStringLibrary.Conv_IntToString` (`self.TargetsLength`))))))

(fn `UserConstructionScript`)