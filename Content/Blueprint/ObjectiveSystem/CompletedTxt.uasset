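; CompletedTxt is a completion indicator for the objective system, celebrating when its referenced objective completes.
; It hides its text render on BeginPlay and binds Update to the objective's completion event.
; When Update fires, it shows the text, then after a short delay activates a confetti particle effect and plays a 2D bubble sound, without checking the Complete value.
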(event `self.ReceiveBeginPlay`
  (`SceneComponent.SetVisibility` (`self.TextRender`) false false)
  (add `/Game/Blueprint/ObjectiveSystem/Objective.ObjectiveComplete` (`self.Objective`) (delegate `Update`)))

(event `Update`
  (params (Objective :type "/Game/Blueprint/ObjectiveSystem/Objective Object Reference") (Complete :type Boolean))
  (`SceneComponent.SetVisibility` (`self.TextRender`) true false)
  (`KismetSystemLibrary.Delay` 0.8)
  (`ActorComponent.SetActive` (`self.P_Confetti`) true false)
  (`GameplayStatics.PlaySound2D` "/Game/Audio/Environment/ES_Bubble_Surface_3.ES_Bubble_Surface_3"))

(fn `UserConstructionScript`)