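; GM_LevelSelect is the level select game mode Blueprint that shows which levels appear in the saved game.
; On BeginPlay it loads the save through GI_GameInstance and toggles each level marker's text render by whether its level name is in the saved data.
; A LoadLevel event takes an array of biome markers and an index, then calls BiomeSelected on the chosen marker.
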(event `self.ReceiveBeginPlay`
  (bind _asgi_game_instance (cast `/Game/Blueprint/Managers/GI_GameInstance` (`GameplayStatics.GetGameInstance`)))
  (bind _levels (`/Game/Blueprint/Managers/GI_GameInstance.LoadGame` _asgi_game_instance))
  (for _array_element (`self.LevelMarkers`)
    (if (`KismetArrayLibrary.Array_Contains` _levels (`KismetStringLibrary.Conv_NameToString` (`/Game/Levels/A_LevelClick.LevelName` _array_element)))
      (bind _textrender (`/Game/Levels/A_LevelClick.TextRender` _array_element))
      (`SceneComponent.SetVisibility` _textrender true false)
      (else
        (`SceneComponent.SetVisibility` _textrender false false)))))

(event `LoadLevel`
  (params (BiomeMarkers :type "Array of /Game/Levels/A_LevelClick Object Reference") (BiomeIndex :type Integer))
  (`/Game/Levels/A_LevelClick.BiomeSelected` (`|GetArrayItem` BiomeMarkers BiomeIndex)))

(fn `UserConstructionScript`)