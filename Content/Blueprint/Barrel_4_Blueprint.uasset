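; Barrel actor Blueprint that re-orients its static mesh every tick from the normal returned by a line trace.
; The trace targets WorldStatic objects, ignores itself, and runs between the relative locations of the Bottom and Arrow components, used directly as trace points.
; The hit normal becomes the mesh's X axis, while world location is kept and scale is forced to a small uniform value.
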(event `self.ReceiveTick`
  (params (DeltaSeconds :type "Float (single-precision)"))
  (bind _outhit (`KismetSystemLibrary.LineTraceSingleForObjects` (`SceneComponent.RelativeLocation` (`self.Bottom`)) (`SceneComponent.RelativeLocation` (`self.Arrow`)) (`|MakeArray` "ObjectTypeQuery1" :!type "EObjectTypeQuery Enum") false (`|MakeArray` self :!type "Actor Object Reference")))
  (`SceneComponent.K2_SetWorldTransform` (`self.StaticMeshComponent`) (`KismetMathLibrary.MakeTransform` (`SceneComponent.K2_GetComponentLocation` (`self.StaticMeshComponent`)) (`KismetMathLibrary.Conv_VectorToRotator` (`.Normal` (`GameplayStatics.BreakHitResult` _outhit))) (0.1 0.1 0.1)) false false))

(fn `UserConstructionScript`)