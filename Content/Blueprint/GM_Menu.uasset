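; GM_Menu is the menu game mode, which sets up the menu UI and its input when play begins.
; It adds the W_MenuControl widget to the player screen, shows the cursor and caches all WA_Menu panels and MenuNode actors in the level.
; The first panel found gets focus in Game and UI input mode, and its widget binds to the first button message.
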(event `self.ReceiveBeginPlay`
  (bind _returnvalue (`GameplayStatics.GetPlayerController` 0))
  (bind _returnvalue_2 (`|CreateWidget` "/Game/Widgets/Menu/W_MenuControl.W_MenuControl_C"))
  (`UserWidget.AddToPlayerScreen` _returnvalue_2 0)
  (set `PlayerController.bShowMouseCursor` true _returnvalue)
  (bind _outactors (`GameplayStatics.GetAllActorsOfClass` "/Game/Widgets/Menu/WA_Menu.WA_Menu_C"))
  (bind _output_get (set `self.MenuPanels` _outactors))
  (bind _returnvalue_3 (`WidgetComponent.GetUserWidgetObject` (`/Game/Widgets/Menu/WA_Menu.Widget` (`|GetArrayItem` _output_get))))
  (`WidgetBlueprintLibrary.SetInputMode_GameAndUIEx` _returnvalue _returnvalue_3)
  (message `/Game/Blueprint/Interfaces/I_Menu.BindToFirstButton` _returnvalue_3)
  (bind _outactors_2 (`GameplayStatics.GetAllActorsOfClass` "/Game/Widgets/Menu/MenuNode.MenuNode_C"))
  (set `self.MenuNodes` _outactors_2))

(fn `UserConstructionScript`)