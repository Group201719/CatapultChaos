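; Game mode for the catapult game that runs a level through pregame, in-game, pause and win or lose screens.
; On init it sets up managers and objectives, then spawns and possesses the player pawn; start loads the GameInstance deck.
; Objective completion events trigger the win check, and zone changes teleport the pawn to that objective's spawn transform.
; Winning scores leftover budget plus half the value of remaining shots.
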(event `/Game/Blueprint/Interfaces/I_Gamemode.SpawnPlayer`
  ;[1 1 1] Gamemode Interface Events
  (`self.SpawnPlayerBP`))

(event `/Game/Blueprint/Interfaces/I_Gamemode.SetupManagers`
  ;[1 1 1] Gamemode Interface Events
  (`self.SetupManagersBP`))

(event `/Game/Blueprint/Interfaces/I_Gamemode.SetupObjectives`
  ;[1 1 1] Gamemode Interface Events
  (bind _outactors (`self.SetupObjectivesBP`))
  (set `self._Objective` _outactors))

(event `/Game/Blueprint/Interfaces/I_Gamemode.CheckObjectives`
  ;[1 1 1] Gamemode Interface Events
  (bind _complete (`self.AreObjectivesCompleteBP`))
  (if _complete
    (`self.EndGame` true)))

(event `/Game/Blueprint/Interfaces/I_Gamemode.GetZoneChange`
  (params (int :type Integer))
  ;[1 1 1] Zone Change Event
  (bind _transform (`self.ZoneChange` int))
  (`self.K2_TeleportTo` (`/Game/Blueprint/Controller/C_PlayerController.OwnedPawn` (`self.Player`)) (.location _transform) (.rotation _transform)))

(event `self.ReceiveBeginPlay`
  ;[1 1 1] BeginPlay
  (`self.Init`))

(event `/Game/Blueprint/Interfaces/I_Gamemode.FillLevelInfo`
  (params (LevelInfo :type "/Game/Blueprint/Managers/LevelInfo Structure"))
  ;[1 1 1] Fill Level Info
  (set `self.LevelInfo` LevelInfo))

(event `ObjectiveComplete`
  (params (Objective :type "/Game/Blueprint/ObjectiveSystem/Objective Object Reference") (Complete :type Boolean))
  ;[1 1 1] Track Objectives and completions
  (bind _complete (`self.AreObjectivesCompleteBP`))
  (if _complete
    (`self.EndGame` true)))

(event `Init`
  ;[1 1 1] Init
  (bind _asc_player_controller (cast `/Game/Blueprint/Controller/C_PlayerController` (`GameplayStatics.GetPlayerController` 0)))
  (set `self.Player` _asc_player_controller)
  (`self.SetupManagersBP`)
  (bind _returnvalue (`|CreateWidget` "/Game/Widgets/W_Pregame.W_Pregame_C" null (`self.LevelInfo`)))
  (`UserWidget.AddToPlayerScreen` _returnvalue 0)
  (`WidgetBlueprintLibrary.SetInputMode_GameAndUIEx` (`self.Player`) (`/Game/Widgets/W_Pregame.B_StartGame` _returnvalue))
  (set `self.GameStates` "NewEnumerator0")
  (bind _outactors (`self.SetupObjectivesBP`))
  (bind _output_get (set `self._Objective` _outactors))
  (for _array_element _output_get
    ;[1 1 1] Track Objectives and completions
    (`/Game/Blueprint/ObjectiveSystem/Objective.Init` _array_element (`/Game/Blueprint/ObjectiveSystem/Objective.Type` _array_element))
    (add `/Game/Blueprint/ObjectiveSystem/Objective.ObjectiveComplete` _array_element (delegate `ObjectiveComplete`)))
  (`self.SpawnPlayerBP`)
  (`AudioComponent.Play` (`self.Audio`) 0.0))

(event `/Game/Blueprint/Interfaces/I_Gamemode.StartGame`
  (bind _player (`self.Player`))
  ;[1 1 1] Start Game
  (`WidgetLayoutLibrary.RemoveAllWidgets`)
  (bind _asgi_game_instance (cast `/Game/Blueprint/Managers/GI_GameInstance` (`GameplayStatics.GetGameInstance`))
    (:`then`
      (bind _return (`/Game/Blueprint/Managers/GI_GameInstance.GetDeck` _asgi_game_instance))
      (`/Game/Blueprint/P_PlayerPawn.LoadCurrentDeck` (`/Game/Blueprint/Controller/C_PlayerController.OwnedPawn` _player) _return)
      (`/Game/Blueprint/Controller/C_PlayerController.LoadSpecificShot` _player (`|GetArrayItem` _return))
      (set `PlayerController.bShowMouseCursor` false (`GameplayStatics.GetPlayerController` 0))
      (set `self.GameStates` "NewEnumerator1")
      (bind _returnvalue (`|CreateWidget` "/Game/Widgets/W_InGame.W_InGame_C"))
      (bind _output_get (set `self.InGameWidget` _returnvalue))
      (`UserWidget.AddToPlayerScreen` _output_get 0)
      (`/Game/Widgets/W_InGame.ChangeObjective` _output_get (`/Game/Blueprint/ObjectiveSystem/Objective.Text` (`|GetArrayItem` (`self._Objective`))))
      (`self.OpenLevelText` (`KismetTextLibrary.Conv_StringToText` (`.IntroText_21_E555E9FD4E45C804F745DAB3CD102883` (break `/Game/Blueprint/Managers/LevelInfo` (`self.LevelInfo`)))))
      (`AudioComponent.Stop` (`self.Audio`))
      (`GameplayStatics.PlaySoundAtLocation` "/Game/Audio/Outro.Outro"))
    (:`CastFailed`
      (`KismetSystemLibrary.PrintString` "Instance Cast Failed"))))

(event `/Game/Blueprint/Interfaces/I_Gamemode.EndGame`
  (params (Win :type Boolean))
  ;[1 1 1] End The game
  (if (`|EnumEquality` (`self.GameStates`) "NewEnumerator1")
    (set `self.GameStates` "NewEnumerator2")
    (if Win
      (`WidgetLayoutLibrary.RemoveAllWidgets`)
      (bind _returnvalue (`|CreateWidget` "/Game/Widgets/W_WinGame.W_WinGame_C"))
      (`UserWidget.AddToPlayerScreen` _returnvalue 0)
      (`self.FinaliseScore`)
      (else
        (`WidgetLayoutLibrary.RemoveAllWidgets`)
        (bind _returnvalue_2 (`|CreateWidget` "/Game/Widgets/W_Endgame.W_Endgame_C"))
        (`UserWidget.AddToPlayerScreen` _returnvalue_2 0)))))

(event `/Game/Blueprint/Interfaces/I_Gamemode.Pause`
  (params (Pause :type Boolean))
  ;[1 1 1] Pause Game
  (switch `/Game/Blueprint/E_GameStates` (`self.GameStates`)
    (:`NewEnumerator1`
      (if Pause
        (`WidgetLayoutLibrary.RemoveAllWidgets`)
        (`GameplayStatics.SetGamePaused` Pause)
        (bind _returnvalue (`|CreateWidget` "/Game/Widgets/W_pauseGame.W_pauseGame_C"))
        (`WidgetBlueprintLibrary.SetInputMode_GameAndUIEx` (`self.Player`) (`/Game/Widgets/W_pauseGame.Button_80` _returnvalue))
        (`UserWidget.AddToPlayerScreen` _returnvalue 0)
        (else
          (`WidgetLayoutLibrary.RemoveAllWidgets`)
          (`GameplayStatics.SetGamePaused` false)
          (bind _returnvalue_2 (`|CreateWidget` "/Game/Widgets/W_InGame.W_InGame_C"))
          (`UserWidget.AddToPlayerScreen` _returnvalue_2 0))))))

(event `/Game/Blueprint/Interfaces/I_Gamemode.DepthTargets`
  (params (Hidden :type Boolean))
  ;[1 1 1] Shit code 101 - change if it works
  (bind _filteredarray (`KismetArrayLibrary.FilterArray` (`self.ActiveManagers`) "/Game/Blueprint/Managers/TargetManager.TargetManager_C"))
  (for _array_element _filteredarray
    (bind _astarget_manager (cast `/Game/Blueprint/Managers/TargetManager` _array_element))
    (`/Game/Blueprint/Managers/TargetManager.LightTargets` _astarget_manager Hidden)))

(event `OpenLevelText`
  (params (Text :type Text))
  ;[1 1 1] LevelOpen
  (`/Game/Widgets/W_InGame.ShowTaunt` (`self.InGameWidget`) Text))

(fn `AreObjectivesCompleteBP`
  (returns (Complete :type Boolean))
  (locals (Completes :type "Array of Boolean"))
  (bind __objective (`self._Objective`))
  (for _array_element __objective
    (if (`/Game/Blueprint/ObjectiveSystem/Objective.Complete` _array_element)
      (`KismetArrayLibrary.Array_Add` (`local.Completes`) true)))
  (if (== (`KismetArrayLibrary.Array_Length` __objective) (`KismetArrayLibrary.Array_Length` (`local.Completes`)))
    (return true)
    (else
      (return false))))

(fn `FinaliseScore`
  (bind _ownedpawn (`/Game/Blueprint/Controller/C_PlayerController.OwnedPawn` (`self.Player`)))
  (bind _currentshotindex (`/Game/Blueprint/P_PlayerPawn.CurrentShotIndex` _ownedpawn))
  (bind _projectilestospawn (`/Game/Blueprint/P_PlayerPawn.ProjectilesToSpawn` _ownedpawn))
  (bind _returnvalue (`KismetArrayLibrary.Array_LastIndex` _projectilestospawn))
  (set `self.FinalScore` (- (`self.LevelBudget`) (`self.TotalSpent`)))
  (if (not (== _currentshotindex _returnvalue))
    (for _index (range _currentshotindex (+ _returnvalue 1))
      (set `self.FinalScore` (+ (`self.FinalScore`) (/ (`.Value_7_08F0D3864924CEB4A733DAA526472BDA` (break `/Game/Blueprint/Projectiles/ProjectileInfo` (defaults `/Game/Blueprint/GM_Tutorial` (`|GetArrayItem` _projectilestospawn _index)))) 2))))))

(fn `GetGameState`
  (returns (GameState :type "/Game/Blueprint/E_GameStates Enum"))
  (return (`self.GameStates`)))

(fn `GetObjectives`
  (returns (Objectives :type "Array of /Game/Blueprint/ObjectiveSystem/Objective Object Reference"))
  (return (`self._Objective`)))

(fn `GetTargetManagers`
  (params (managersIn :type "Array of /Game/Blueprint/BaseManager Object Reference (by ref)"))
  (returns (Managers :type "Array of /Game/Blueprint/Managers/TargetManager Object Reference"))
  (return))

(fn `SetupManagersBP`
  (returns (ActiveManagers :type "Array of /Game/Blueprint/BaseManager Object Reference"))
  (locals (Tempmanagers :type "Array of /Game/Blueprint/BaseManager Object Reference"))
  (bind _outactors (`GameplayStatics.GetAllActorsWithInterface` "/Game/Blueprint/Interfaces/I_Managers.I_Managers_C"))
  (for _array_element _outactors
    (message `/Game/Blueprint/Interfaces/I_Managers.Init` _array_element)
    (bind _asbase_manager (cast `/Game/Blueprint/BaseManager` _array_element))
    (`KismetArrayLibrary.Array_Add` (`local.Tempmanagers`) _asbase_manager))
  (bind _output_get (set `self.ActiveManagers` (`local.Tempmanagers`)))
  (return _output_get))

(fn `SetupObjectivesBP`
  (returns (OutActors :type "Array of /Game/Blueprint/ObjectiveSystem/Objective Object Reference"))
  (locals (Objectives :type "Array of /Game/Blueprint/ObjectiveSystem/Objective Object Reference"))
  (bind _outactors (`GameplayStatics.GetAllActorsWithInterface` "/Game/Blueprint/ObjectiveSystem/IObjective.IObjective_C"))
  (for _array_element _outactors
    (bind _asobjective (cast `/Game/Blueprint/ObjectiveSystem/Objective` _array_element))
    (`KismetArrayLibrary.Array_Add` (`local.Objectives`) _asobjective))
  (return (`local.Objectives`)))

(fn `SpawnPlayerBP`
  (bind _player (`self.Player`))
  (bind _transform (`self.ZoneChange` 1))
  (bind _returnvalue (`|SpawnActorFromClass` "/Game/Blueprint/P_PlayerPawn.P_PlayerPawn_C" _transform "Undefined" "OverrideRootScale" null "100.000000,100.000000,100.000000|-0.000014,-179.999969,-179.999969|1.000000,1.000000,1.000000" null))
  (bind _output_get (set `/Game/Blueprint/Controller/C_PlayerController.OwnedPawn` _returnvalue _player))
  (`/Game/Blueprint/Controller/C_PlayerController.Init` _player)
  (`/Game/Blueprint/P_PlayerPawn.Init` _output_get)
  (`Controller.Possess` _player _output_get)
  (set `/Game/Blueprint/Controller/C_PlayerController.CurrentPoint` 1 _player)
  (return))

(fn `Taunt`
  (params (ProjectileName :type "Actor Class Reference") (Widget :type "/Game/Widgets/W_InGame Object Reference"))
  (switch `string` (`KismetSystemLibrary.GetClassDisplayName` ProjectileName)))

(fn `UserConstructionScript`)

(fn `ZoneChange`
  (params (ChangeTo :type Integer))
  (returns (Transform :type "Transform Structure"))
  (for _array_element (`self._Objective`)
    (if (== (`/Game/Blueprint/ObjectiveSystem/Objective.Number` _array_element) ChangeTo)
      (return (`/Game/Blueprint/ObjectiveSystem/Objective.SpawnTransform` _array_element))))
  (return))