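; Level select controller that moves the controlled pawn between level markers and loads the chosen one.
; BeginPlay takes the LevelSelectManager's LevelClickActors and snaps the pawn to the first marker's Arrow transform.
; Right mouse or CannonSlot2 advances the index, wrapping at the end, and timelines lerp the pawn from its current transform to that Arrow.
; Select passes the markers and index to GM_LevelSelect's LoadLevel.
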(event `self.ReceiveBeginPlay`
  (bind _arrow (`/Game/Levels/A_LevelClick.Arrow` (`|GetArrayItem` (`self.Targets`))))
  ;[1 1 1] Init
  (bind _outactors (`GameplayStatics.GetAllActorsOfClass` "/Game/Blueprint/Managers/LevelSelectManager.LevelSelectManager_C"))
  (set `self.Targets` (`/Game/Blueprint/Managers/LevelSelectManager.LevelClickActors` (`|GetArrayItem` _outactors)))
  (`self.K2_SetActorTransform` (`self.K2_GetPawn`) (`KismetMathLibrary.MakeTransform` (`SceneComponent.K2_GetComponentLocation` _arrow) (`SceneComponent.K2_GetComponentRotation` _arrow)) true false))

(event `Key|RightMouseButton`
  (params (Key :type "Key Structure"))
  (bind _returnvalue (`self.K2_GetPawn`))
  ;[1 1 1] Inputs
  (:`Pressed`
    (bind _result (`/Engine/EditorBlueprintResources/StandardMacros.IncrementInt` (`self.Length`) :!label _label)
      (:`  `
        (if (>= (`self.Length`) (`KismetArrayLibrary.Array_Length` (`self.Targets`)))
          ;[1 1 1] Reset length then lerp
          (bind _output_get (set `self.Length` 0))
          (bind (_direction _l) (`Timeline|Timeline_1` :!via `PlayFromStart`)
            (:`Update`
              (bind _arrow (`/Game/Levels/A_LevelClick.Arrow` (`|GetArrayItem` (`self.Targets`) _output_get)))
              (`self.K2_SetActorTransform` (`self.K2_GetPawn`) (`KismetMathLibrary.TLerp` (`self.GetTransform` (`self.K2_GetPawn`)) (`KismetMathLibrary.MakeTransform` (`SceneComponent.K2_GetComponentLocation` _arrow) (`SceneComponent.K2_GetComponentRotation` _arrow)) _l) true false)))
          (else
            ;[1 1 1] Lerp To Next Point In sequence
            (bind (_direction_2 _l_2) (`Timeline|Timeline_0` :!via `PlayFromStart`)
              (:`Update`
                (bind _arrow_2 (`/Game/Levels/A_LevelClick.Arrow` (`|GetArrayItem` (`self.Targets`) _result)))
                (`self.K2_SetActorTransform` _returnvalue (`KismetMathLibrary.TLerp` (`self.GetTransform` _returnvalue) (`KismetMathLibrary.MakeTransform` (`SceneComponent.K2_GetComponentLocation` _arrow_2) (`SceneComponent.K2_GetComponentRotation` _arrow_2)) _l_2) true false)))))))))

(event `InputAction|CannonSlot2`
  (params (Key :type "Key Structure"))
  ;[1 1 1] Inputs
  (:`Pressed`
    (goto _label)))

(event `InputAction|Select`
  (params (Key :type "Key Structure"))
  (:`Pressed`
    (bind _asgm_level_select (cast `/Game/Blueprint/GM_LevelSelect` (`GameplayStatics.GetGameMode`)))
    (`/Game/Blueprint/GM_LevelSelect.LoadLevel` _asgm_level_select (`self.Targets`) (`self.Length`))))

(fn `UserConstructionScript`)