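; A test actor that sets off a timed explosion, applying a radial impulse and destructible damage at its location.
; The construction script copies the exposed damage and radius values onto the RadialForce component.
; On BeginPlay a timer calls Detonate after the configured delay, which fires the impulse and plays a catapult sound at the actor's location.
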(event `self.ReceiveBeginPlay`
  (`KismetSystemLibrary.K2_SetTimer` null "Detonate" (`self.DetonationTimer`)))

(fn `Detonate`
  (`RadialForceComponent.FireImpulse` (`self.RadialForce`))
  (`GameplayStatics.PlaySoundAtLocation` "/Game/FirstPersonBP/Catapultwav.Catapultwav" (`self.K2_GetActorLocation`)))

(fn `UserConstructionScript`
  (bind _radialforce (`self.RadialForce`))
  (set `RadialForceComponent.DestructibleDamage` (`self.ExplosionDamage`) _radialforce)
  (set `RadialForceComponent.Radius` (`self.ExplosionRadius`) _radialforce))