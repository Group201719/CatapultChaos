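; LevelManager is an actor Blueprint that hands its level information to the tutorial game mode.
; Its Init event casts the current game mode to GM_Tutorial and passes LevelInfo to FillLevelInfo, doing nothing if the cast fails.
; BeginPlay, overlap and Tick are disabled stubs, so the actor does not call Init itself.
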(event `/Game/Blueprint/Interfaces/I_Managers.Init`
  (bind _asgm_tutorial (cast `/Game/Blueprint/GM_Tutorial` (`GameplayStatics.GetGameMode`)))
  (`/Game/Blueprint/GM_Tutorial.FillLevelInfo` _asgm_tutorial (`self.LevelInfo`)))

(fn `UserConstructionScript`
  (`parent.UserConstructionScript`))