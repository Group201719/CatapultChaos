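; Manager actor that tracks a set of hittable Targets for an owning objective in what appears to be a catapult game.
; Construction script copies Targets into ActiveTargets, and Init initializes each target and binds its hit to TargetHit.
; Each hit removes the target from ActiveTargets, updates objective text and calls the objective's completion check once all targets are hit.
; LightTargets toggles depth status on every target.
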(event `/Game/Blueprint/Interfaces/I_Managers.Init`
  (bind _targets (`self.Targets`))
  (for _array_element _targets
    (`/Game/Blueprint/Target.Init` _array_element)
    (add `/Game/Blueprint/Target.ActorHit` _array_element (delegate `TargetHit`)))
  (set `self.TargetNum` (`KismetArrayLibrary.Array_Length` _targets)))

(event `self.ReceiveBeginPlay`
  (`parent.ReceiveBeginPlay`))

(event `TargetHit`
  (params (hit :type Boolean) (Actor :type "/Game/Blueprint/Target Object Reference") (Projectile :type "Actor Object Reference"))
  (bind _owningobjective (`self.OwningObjective`))
  (`KismetArrayLibrary.Array_RemoveItem` (`self.ActiveTargets`) Actor)
  (`/Game/Blueprint/ObjectiveSystem/Objective.UpdateText` _owningobjective)
  (bind _targetscomplete (`self.CheckIfTargetsCompleted`))
  (if _targetscomplete
    (`/Game/Blueprint/ObjectiveSystem/Objective.IsObjectiveComplete` _owningobjective)))

(fn `CheckIfTargetsCompleted`
  (returns (TargetsComplete :type Boolean) (TargetsCurrentlyHit :type Integer))
  (locals (Temptargets :type "Array of /Game/Blueprint/Target Object Reference"))
  (for _array_element (`self.Targets`)
    (if (`/Game/Blueprint/Target.Hit` _array_element)
      (`KismetArrayLibrary.Array_Add` (`local.Temptargets`) _array_element)))
  (if (== (`KismetArrayLibrary.Array_Length` (`self.Targets`)) (`KismetArrayLibrary.Array_Length` (`local.Temptargets`)))
    (return true (`KismetArrayLibrary.Array_Length` (`local.Temptargets`)))))

(fn `LightTargets`
  (params (Bool :type Boolean))
  (for _array_element (`self.Targets`)
    (`/Game/Blueprint/Target.ChangeDepthStatus` _array_element Bool))
  (return))

(fn `SetOwningObjective`
  (params (Objective :type "/Game/Blueprint/ObjectiveSystem/Objective Object Reference"))
  (returns (Compete :type Boolean))
  (if (`KismetSystemLibrary.IsValid` Objective)
    (set `self.OwningObjective` Objective)
    (return true)
    (else
      (return false))))

(fn `UserConstructionScript`
  (`parent.UserConstructionScript`)
  (for _array_element (`self.Targets`)
    (`KismetArrayLibrary.Array_AddUnique` (`self.ActiveTargets`) _array_element)))