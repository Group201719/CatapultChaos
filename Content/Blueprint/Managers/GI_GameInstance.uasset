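; Game instance that holds the player's deck and tracks completed levels across level loads.
; Init creates a fresh SG_SaveGame and immediately writes it to FirstSlot, overwriting any existing save without loading it.
; SaveGame appends non-empty level entries and saves to the object's own SlotName, while LoadGame reads completed levels from FirstSlot.
; The deck stays in memory only, accessed through GetDeck, SaveDeck and SaveDeckEvent.
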(event `self.ReceiveInit`
  (bind _returnvalue (`GameplayStatics.CreateSaveGameObject` "/Game/SG_SaveGame.SG_SaveGame_C"))
  (bind _output_get (set `self.SaveObject` _returnvalue))
  (set `/Game/SG_SaveGame.CompletedLvls` (`self.CompletedLvl`) _output_get)
  (`GameplayStatics.SaveGameToSlot` _output_get "FirstSlot" 1))

(event `SaveDeckEvent`
  (params (Deck :type "Array of /Game/Blueprint/Projectiles/A_Stone Class Reference"))
  (`self.SaveDeck` Deck))

(fn `GetDeck`
  (returns (return :type "Array of /Game/Blueprint/Projectiles/A_Stone Class Reference"))
  (return (`self.Deck`)))

(fn `LoadGame`
  (returns (levels :type "Array of String"))
  (`self.SaveObject`
    (:`then`
      (bind _returnvalue (`GameplayStatics.LoadGameFromSlot` "FirstSlot" 1))
      (bind _assg_save_game (cast `/Game/SG_SaveGame` _returnvalue))
      (bind _output_get (set `self.CompletedLvl` (`/Game/SG_SaveGame.CompletedLvls` _assg_save_game)))
      (return _output_get))
    (:`else`)))

(fn `SaveDeck`
  (params (_Deck :type "Array of /Game/Blueprint/Projectiles/A_Stone Class Reference"))
  (set `self.Deck` _Deck))

(fn `SaveGame`
  (params (LevelToAdd :type String))
  (bind _saveobject (`self.SaveObject`))
  (if (not (`KismetTextLibrary.TextIsEmpty` (`KismetTextLibrary.Conv_StringToText` LevelToAdd)))
    (`KismetArrayLibrary.Array_Add` (`self.CompletedLvl`) LevelToAdd)
    (`/Engine/EditorBlueprintResources/StandardMacros.IsValid` _saveobject
      (:`Is Valid`
        (set `/Game/SG_SaveGame.CompletedLvls` (`self.CompletedLvl`) _saveobject)
        (`GameplayStatics.SaveGameToSlot` _saveobject (`/Game/SG_SaveGame.SlotName` _saveobject) 1)))))