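; Villager manager actor that gathers the level's villagers and can generate random villager identities.
; Four seconds after BeginPlay, it gets the target managers from the GameMode through an interface message and appends their Targets to Villagers.
; GenerateName builds a villager struct from random name, backstory, age, occupation and sex, with first name chosen independently of sex.
; GenerateName is called only in disconnected debug code, and FillTargets is an empty stub.
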(event `self.ReceiveBeginPlay`
  (`KismetSystemLibrary.Delay` 4.0)
  (bind _managers (message `/Game/Blueprint/Interfaces/I_Gamemode.GetTargetManagers` (`GameplayStatics.GetGameMode`) (`|MakeArray` null :!type "/Game/Blueprint/BaseManager Object Reference")))
  (for _array_element _managers
    (`KismetArrayLibrary.Array_Append` (`self.Villagers`) (`/Game/Blueprint/Managers/TargetManager.Targets` _array_element))))

(event `FillTargets`)

(fn `GenerateName`
  (returns (Info :type "/Game/Blueprint/Managers/Villager Structure"))
  (bind _lastnames (`self.LastNames`))
  (bind _backstories (`self.BackStories`))
  (bind _firstnames (`self.FirstNames`))
  (return (make `/Game/Blueprint/Managers/Villager` (`|GetArrayItem` _firstnames (`KismetMathLibrary.RandomIntegerInRange` 0 (- (`KismetArrayLibrary.Array_Length` _firstnames) 1))) (`|GetArrayItem` _lastnames (`KismetMathLibrary.RandomIntegerInRange` 0 (- (`KismetArrayLibrary.Array_Length` _lastnames) 1))) (`KismetMathLibrary.RandomIntegerInRange` 15 65) (cast `/Game/Blueprint/Managers/Occupations` (`KismetMathLibrary.Conv_IntToByte` (`KismetMathLibrary.RandomIntegerInRange` 0 (- (enumcount `/Game/Blueprint/Managers/Occupations`) 1)))) (`KismetMathLibrary.RandomBool`) (`|GetArrayItem` _backstories (`KismetMathLibrary.RandomIntegerInRange` 0 (- (`KismetArrayLibrary.Array_Length` _backstories) 1))))))

(fn `UserConstructionScript`
  (`parent.UserConstructionScript`))