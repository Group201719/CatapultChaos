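; Villager target actor with an animated arrow marker that dies when struck by a projectile, a fast-moving destructible, or its own high velocity.
; TargetHit enables skeletal mesh physics and, once, broadcasts ActorHit, plays a death cry and hides the arrow.
; Its ActorHit handler messages the A_Stone projectile, briefly shows a death-cam widget with VillagerManager-generated info and shakes the camera.
; AffectGravity also triggers the hit, disabling gravity and pushing the body.
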(event `/Game/Blueprint/Interfaces/I_Gravity.AffectGravity`
  (params (ProjectileVector :type "Vector Structure"))
  (bind _returnvalue (`self.K2_GetActorLocation`))
  (bind _skeletalmesh (`self.SkeletalMesh`))
  (`self.TargetHit`)
  (`PrimitiveComponent.SetEnableGravity` _skeletalmesh false)
  (`PrimitiveComponent.AddForce` _skeletalmesh (`KismetMathLibrary.Normal` (`KismetMathLibrary.GetDirectionUnitVector` ProjectileVector _returnvalue)) "None" false)
  (`GameplayStatics.PlaySoundAtLocation` "/Game/Audio/GravityScream.GravityScream" _returnvalue))

(event `/Game/Blueprint/Interfaces/I_Gravity.DisableGravity`
  (`PrimitiveComponent.SetEnableGravity` (`self.SkeletalMesh`) true))

(event `TargetHit`
  (bind _deathnoise (`self.DeathNoise`))
  (set `self.Hit` true)
  (`PrimitiveComponent.SetSimulatePhysics` (`self.SkeletalMesh`) true)
  (`PrimitiveComponent.SetCollisionEnabled` (`self.SkeletalMesh`) "QueryAndPhysics")
  (`/Engine/EditorBlueprintResources/StandardMacros.DoOnce` false
    (:`Completed`
      (`self.ActorHit` (`self.Hit`) self (`self.Projectile Reference`))
      (`GameplayStatics.PlaySoundAtLocation` (`|GetArrayItem` _deathnoise (`KismetMathLibrary.RandomIntegerInRange` 0 (`KismetArrayLibrary.Array_Length` _deathnoise))) (`SceneComponent.K2_GetComponentLocation` (`self.Arrow`)) (struct) 1.0 (`GameplayStatics.GetGlobalTimeDilation`))
      (`SceneComponent.SetVisibility` (`self.ArrowMesh`) false false))))

(event `self.Box.OnComponentHit`
  (params (HitComponent :type "PrimitiveComponent Object Reference") (OtherActor :type "Actor Object Reference") (OtherComp :type "PrimitiveComponent Object Reference") (NormalImpulse :type "Vector Structure") (Hit :type "HitResult Structure (by ref)"))
  (bind _returnvalue (`GameplayStatics.GetGlobalTimeDilation`))
  (`/Engine/EditorBlueprintResources/StandardMacros.IsValid` OtherActor
    (:`Is Valid`
      (if (`self.Hit`)
        _
        (elif (or (`KismetSystemLibrary.DoesImplementInterface` OtherActor "/Game/Blueprint/Interfaces/I_Projectile.I_Projectile_C") (and (`KismetSystemLibrary.DoesImplementInterface` OtherActor "/Game/Blueprint/Interfaces/I_Destructible.I_Destructible_C") (>= (`KismetMathLibrary.VSize` (`self.GetVelocity` OtherActor)) (`self.Physicsthreshhold`))))
          (`GameplayStatics.PlaySound2D` "/Game/PhysicalMaterials/FX/FleshSurface1.FleshSurface1" 0.3 _returnvalue)
          (`GameplayStatics.PlaySound2D` "/Game/PhysicalMaterials/BoneCrunch.BoneCrunch" 0.3 _returnvalue)
          (set `self.Projectile Reference` OtherActor)
          (`self.TargetHit` :!label _label))))))

(event `self.ReceiveTick`
  (params (DeltaSeconds :type "Float (single-precision)"))
  (bind _physicsthreshhold (`self.Physicsthreshhold`))
  (bind _returnvalue (`PrimitiveComponent.GetPhysicsLinearVelocity` (`self.Box`) "None"))
  (if (or (> (.x _returnvalue) _physicsthreshhold) (> (.y _returnvalue) _physicsthreshhold) (> (.z _returnvalue) _physicsthreshhold))
    (goto _label)))

(event `self.ReceiveBeginPlay`
  (bind (_direction _arrow_move) (`Timeline|ArrowMove`)
    (:`Update`
      (`SceneComponent.K2_SetRelativeLocation` (`self.ArrowMesh`) _arrow_move false false)
      (add `self.ActorHit` (delegate `Camera Switch`)))))

(event `Camera Switch` :!signature `self.ActorHit`
  (params (hit :type Boolean) (Actor :type "/Game/Blueprint/Target Object Reference") (Projectile :type "Actor Object Reference"))
  (if (== Actor self)
    (bind _asa_stone (cast `/Game/Blueprint/Projectiles/A_Stone` Projectile))
    (message `/Game/Blueprint/Interfaces/I_Projectile.Death Cam` _asa_stone self)
    (bind _returnvalue (`|CreateWidget` "/Game/Widgets/W_DeathCam.W_DeathCam_C"))
    (message `/Game/Blueprint/Interfaces/I_Player.Get Vilager Info` _returnvalue (`self.Villager_info`))
    (`UserWidget.AddToViewport` _returnvalue 0)
    (`GameplayStatics.PlayWorldCameraShake` "/Game/My_CameraShake.My_CameraShake_C" (`SceneComponent.K2_GetComponentLocation` (`self.Box`)) 0.0 2000.0)
    (`KismetSystemLibrary.Delay` 1.5)
    (`Widget.RemoveFromParent` _returnvalue)))

(fn `ChangeDepthStatus`
  (params (IsHidden :type Boolean))
  (if IsHidden
    (`SceneComponent.SetHiddenInGame` (`self.ArrowMesh`) IsHidden false)
    (else
      (`SceneComponent.SetHiddenInGame` (`self.ArrowMesh`) IsHidden false))))

(fn `Init`
  (bind _outactors (`GameplayStatics.GetAllActorsOfClass` "/Game/Blueprint/Managers/VillagerManager.VillagerManager_C"))
  (bind _info (`/Game/Blueprint/Managers/VillagerManager.GenerateName` (`|GetArrayItem` _outactors)))
  (set `self.Villager_info` _info))

(fn `UserConstructionScript`
  (for _array_element (`self.GetComponentsByTag` "/Script/Engine.ArrowComponent" "Camera")
    (`KismetArrayLibrary.Array_Add` (`self.Camera Array`) _array_element)))