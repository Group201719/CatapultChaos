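; Player controller for a catapult game, forwarding traverse, elevation and firing input to the owned pawn, gated by game state.
; Holding the power axis runs a timeline that sets fire power; release triggers the catapult AnimBP, while Fire launches the shot with that power.
; A secondary action toggles a timeline-lerped overhead camera that blocks aiming.
; Check helpers guard input and ammo, telling the game mode to end the game when ammo runs out.
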(event Input|ActionEvents|InputActionCannonSlot1
  (params (Key :type Key%20Structure))
  ;[1 1 1] Change to Next Projectile
)

(event Input|ActionEvents|InputActionDebugFire
  (params (Key :type Key%20Structure))
  ;[1 1 1] DEBUG
  (:Pressed
    (if (stale Input|AxisEvents|InputAxisPowerWeapon _bool)
      (Utilities|CheckCanFire
        (:CanFire
          (Default|Fire (Variables|Default|GetOwnedPawn) 0.0)
          (Variables|Default|SetCanInput false)
          (Audio|PlaySoundatLocation "/Game/FirstPersonBP/Catapultwav.Catapultwav" (Transformation|GetActorLocation (Variables|Default|GetOwnedPawn))))
        (:OutOfAmmo
          (if (stale _bool)
            (Class|IGamemode|EndGame(Message) (Game|GetGameMode) false)))))))

(event Input|ActionEvents|InputActionSecondaryAction
  (params (Key :type Key%20Structure))
  (bind _returnvalue (Game|GetGameMode))
  (bind _ownedpawn (Variables|Default|GetOwnedPawn))
  (bind _camera (Variables|/Game/Blueprint/P_PlayerPawn.P_PlayerPawn_C|GetCamera _ownedpawn))
  ;[1 1 1] Overhead Camera
  ;;[1 1 1] Pre Movement Checks
  (:Pressed
    (if (stale _bool)
      (if (not (Variables|Default|GetIsFiring))
        (bind _output_get (Variables|Default|SetOverhead (not (Variables|Default|GetOverhead))))
        (if _output_get
          (if (Variables|Default|GetCanInput)
            (Variables|Default|SetCanInput false)
            (Variables|Default|SetCameraTransform (Transformation|GetWorldTransform _camera))
            (bind _movement (Timeline|CameraMovement Play)
              (:Update
                (Transformation|SetWorldTransform _camera (Math|Transform|Lerp(Transform) (Variables|Default|GetCameraTransform) (Variables|/Game/Blueprint/P_PlayerPawn.P_PlayerPawn_C|GetCameraTopPoint _ownedpawn) _movement) false false))
              (:Finished
                (Variables|Default|SetCanInput true)
                ;[1 1 1] Shit code 2.0
                (Utilities|FlowControl|FlipFlop
                  (:A
                    (Class|IGamemode|DepthTargets(Message) _returnvalue false))
                  (:B
                    (Class|IGamemode|DepthTargets(Message) _returnvalue true)))))
            (else
              (Timeline|CameraMovement Play)))
          (elif (Variables|Default|GetCanInput)
            (Variables|Default|SetCanInput false)
            (Timeline|CameraMovement Reverse)
            (else
              (Timeline|CameraMovement Reverse))))))))

(event Input|AxisEvents|InputAxisPowerWeapon
  (params (AxisValue :type Float%20%28single-precision%29))
  ;[1 1 1] Fire
  (bind _bool (Utilities|CheckGameState "NewEnumerator1")
    (:Out
      (if _bool
        (Utilities|CheckCanFire
          (:CanFire
            (if (< AxisValue 0.0)
              (Variables|Default|SetFireHeld true)
              (bind _firepower (Timeline|T_FirePower Play)
                (:Update
                  (Variables|Default|SetFirePower _firepower)
                  (Variables|Default|SetMovementPower _firepower))
                (:Finished
                  (Variables|Default|SetFirePower 0.0)
                  (Variables|Default|SetMovementPower 0.0)))
              (elif (Variables|Default|GetFireHeld)
                (Default|Fire (Variables|Default|GetAnimationBP))
                (Timeline|T_FirePower Stop)))))))))

(event Input|AxisEvents|InputAxisTraverseGun
  (params (AxisValue :type Float%20%28single-precision%29))
  ;[1 1 1] Handle Traverse/Elevation
  (bind _bool (Utilities|CheckGameState "NewEnumerator1")
    (:Out
      (if (and _bool (not (Variables|Default|GetOverhead)))
        (Default|TraverseGun (Variables|Default|GetOwnedPawn) AxisValue)))))

(event Input|AxisEvents|InputAxisElevateGun
  (params (AxisValue :type Float%20%28single-precision%29))
  ;[1 1 1] Handle Traverse/Elevation
  (bind _bool (Utilities|CheckGameState "NewEnumerator1")
    (:Out
      (if (and (not (Variables|Default|GetOverhead)) _bool)
        (Default|ElevateGun (Variables|Default|GetOwnedPawn) AxisValue)))))

(fn ConstructionScript)

(fn Init
  (bind _outactors (Actor|GetAllActorsOfClass "/Game/Blueprint/CameraPoint.CameraPoint_C"))
  (Variables|Default|SetCameraMovePoints _outactors)
  (bind _asanim_bp_catapult (Utilities|Casting|CastToAnimBP_Catapult (Components|SkeletalMesh|GetAnimInstance (Variables|/Game/Blueprint/P_PlayerPawn.P_PlayerPawn_C|GetCatapultMesh (Variables|Default|GetOwnedPawn)))))
  (Variables|Default|SetAnimationBP _asanim_bp_catapult)
  (CallFunction|ResetFire)
  (return))

(fn AddFirePower
  (bind _output_get (Variables|Default|SetFirePower (Math|Float|Clamp(Float) (- (Variables|Default|GetMovementPower) (Variables|Default|GetFireDecayRate)) -1.0 0.0)))
  (Variables|Default|SetMovementPower (Math|Float|Clamp(Float) (- (Variables|Default|GetMovementPower) (Variables|Default|GetFireDecayRate)) -1.0 0.0)))

(fn Fire
  (Default|Fire (Variables|Default|GetOwnedPawn) (Variables|Default|GetMovementPower) self)
  (Variables|Default|SetCanInput false)
  (Audio|PlaySoundatLocation "/Game/FirstPersonBP/Catapultwav.Catapultwav" (Transformation|GetActorLocation (Variables|Default|GetOwnedPawn)))
  (Variables|Default|SetFireHeld false)
  (Variables|Default|SetMovementPower 0.0)
  (Variables|Default|SetFirePower 0.0)
  (Utilities|Time|ClearandInvalidateTimerbyHandle (Variables|Default|GetPowerDecayTimerHandle))
  (Class|ForceFeedbackComponent|SetIntensityMultiplier (Variables|Default|GetForceFeedback) 0.0)
  (Utilities|CheckAmmo
    (:OutOfAmmo
      (Class|IGamemode|EndGame(Message) (Game|GetGameMode) false))))

(fn ResetFire
  (bind _animationbp (Variables|Default|GetAnimationBP))
  (Variables|Default|SetIsFiring false)
  (Variables|Default|SetCanInput true)
  (Variables|/Game/art/Catapult/Animations/AnimBP_Catapult.AnimBP_Catapult_C|SetCurrentAnimation _animationbp "/Game/art/Catapult/Animations/Anim_Catapult_Charge.Anim_Catapult_Charge")
  (Variables|/Game/art/Catapult/Animations/AnimBP_Catapult.AnimBP_Catapult_C|SetReloading _animationbp false)
  (Variables|/Game/art/Catapult/Animations/AnimBP_Catapult.AnimBP_Catapult_C|SetCharging _animationbp true)
  (CallFunction|CheckEnd))

(fn LoadSpecificShot
  (params (ShotToLoad :type A%20Stone%20Class%20Reference))
  (Variables|/Game/Blueprint/P_PlayerPawn.P_PlayerPawn_C|SetNextProjectile (Variables|Default|GetOwnedPawn) ShotToLoad))

(fn CheckEnd
  (Utilities|CheckEndGame))