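; Tutorial controller for the catapult that cycles through practice zones, each loading its own projectile type.
; The cannon slot inputs step CurrentPoint and notify the game mode, then CheckNext maps the zone to a shot.
; Fire launches from the pawn, resets power and feedback, then reloads or ends the game when ammo runs out.
; Other inputs toggle pause and Target depth display; gun axis events are empty and widget highlighting is disconnected.
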(event `InputAction|CannonSlot1`
  (params (Key :type "Key Structure"))
  (bind _returnvalue (`GameplayStatics.GetGameMode`))
  (bind _currentpoint (`self.CurrentPoint`))
  ;[1 1 1] In need of macro - CONTOLS SWITCHING ZONES
  (:`Pressed`
    (bind _objectives (message `/Game/Blueprint/Interfaces/I_Gamemode.GetObjectives` _returnvalue))
    (if (<= _currentpoint 0)
      (set `self.CurrentPoint` 9)
      (message `/Game/Blueprint/Interfaces/I_Gamemode.GetZoneChange` _returnvalue (stale _result) :!label _label)
      (`self.CheckNext`)
      (else
        (bind _result (`/Engine/EditorBlueprintResources/StandardMacros.DecrementInt` _currentpoint)
          (:`  `
            (if (<= _result 0)
              (`/Engine/EditorBlueprintResources/StandardMacros.IncrementInt` _result)
              (else
                (goto _label)))))))))

(event `InputAction|CannonSlot2`
  (params (Key :type "Key Structure"))
  (bind _returnvalue (`GameplayStatics.GetGameMode`))
  (bind _currentpoint (`self.CurrentPoint`))
  ;[1 1 1] In need of macro - CONTOLS SWITCHING ZONES
  (:`Pressed`
    (bind _objectives (message `/Game/Blueprint/Interfaces/I_Gamemode.GetObjectives` _returnvalue))
    (if (>= _currentpoint (`KismetArrayLibrary.Array_Length` _objectives))
      (set `self.CurrentPoint` 1)
      (else
        (bind _result (`/Engine/EditorBlueprintResources/StandardMacros.IncrementInt` _currentpoint)
          (:`  `
            _))))
    (message `/Game/Blueprint/Interfaces/I_Gamemode.GetZoneChange` _returnvalue _result)
    (`self.CheckNext`)))

(event `InputAxis|ElevateGun` :overrideparent false
  (params (AxisValue :type "Float (single-precision)")))

(event `InputAxis|TraverseGun` :overrideparent false
  (params (AxisValue :type "Float (single-precision)")))

(event `InputAxis|PowerWeapon` :consume false :overrideparent false
  (params (AxisValue :type "Float (single-precision)")))

(event `InputAction|Action` :consume false :overrideparent false
  (params (Key :type "Key Structure")))

(event `InputAction|DebugFire` :paused true
  (params (Key :type "Key Structure"))
  (bind _returnvalue (`GameplayStatics.GetGameMode`))
  (:`Pressed`
    (bind _isa (`/Engine/EditorBlueprintResources/StandardMacros.FlipFlop`)
      (:`A`
        (message `/Game/Blueprint/Interfaces/I_Gamemode.Pause` _returnvalue _isa))
      (:`B`
        (message `/Game/Blueprint/Interfaces/I_Gamemode.Pause` _returnvalue false)))))

(event `self.Fire`
  (`/Game/Blueprint/P_PlayerPawn.Fire` (`self.OwnedPawn`) (`self.MovementPower`) self)
  (set `self.CanInput` false)
  (`GameplayStatics.PlaySoundAtLocation` "/Game/FirstPersonBP/Catapultwav.Catapultwav" (`self.K2_GetActorLocation` (`self.OwnedPawn`)))
  (set `self.FireHeld` false)
  (set `self.MovementPower` 0.0)
  (set `self.FirePower` 0.0)
  (`KismetSystemLibrary.K2_ClearAndInvalidateTimerHandle` (`self.PowerDecayTimerHandle`))
  (`ForceFeedbackComponent.SetIntensityMultiplier` (`self.ForceFeedback`) 0.0)
  (`self.CheckAmmo`
    (:`OutOfAmmo`
      (message `/Game/Blueprint/Interfaces/I_Gamemode.EndGame` (`GameplayStatics.GetGameMode`) false))
    (:`AmmoRemaining`
      (`self.CheckNext`))))

(event `InputAction|SecondaryAction` :overrideparent false
  (params (Key :type "Key Structure"))
  (:`Pressed`
    (bind _outactors (`GameplayStatics.GetAllActorsOfClass` "/Game/Blueprint/Target.Target_C"))
    (for _array_element _outactors
      (if (`self.Arrow Hidden?`)
        (`/Game/Blueprint/Target.ChangeDepthStatus` _array_element false)
        (else
          (`/Game/Blueprint/Target.ChangeDepthStatus` _array_element true))))
    (if (`self.Arrow Hidden?`)
      (set `self.Arrow Hidden?` false)
      (else
        (set `self.Arrow Hidden?` true)))))

(fn `UserConstructionScript`
  (`parent.UserConstructionScript`))