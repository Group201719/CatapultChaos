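; Tutorial game mode that overrides the parent's init, game start and player spawn events.
; Init copies the tutorial flag from LevelInfo, and the spawn override creates, initializes and possesses the player pawn at the transform from ZoneChange.
; Game start loads the chicken shot with near-unlimited ammo, hides the cursor, and opens the in-game HUD with the first objective and the level intro text.
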(event `self.Init`
  ;[1 1 1] Init Override
  (`parent.Init`)
  (set `self.IsTutorial` (`.IsTutorial?_18_7AFF98034060C6BEA66A5E9A4A83C5F5` (break `/Game/Blueprint/Managers/LevelInfo` (`self.LevelInfo`)))))

(event `/Game/Blueprint/Interfaces/I_Gamemode.StartGame`
  (bind _player (`self.Player`))
  ;[1 1 1] Start Game Override
  (`WidgetLayoutLibrary.RemoveAllWidgets`)
  (cast `/Game/Blueprint/Managers/GI_GameInstance` (`GameplayStatics.GetGameInstance`)
    (:`then`
      (`/Game/Blueprint/Controller/C_PlayerController.LoadSpecificShot` _player "/Game/Blueprint/Projectiles/A_Chicken.A_Chicken_C")
      (set `/Game/Blueprint/P_PlayerPawn.Ammo` 999 (`/Game/Blueprint/Controller/C_PlayerController.OwnedPawn` _player))
      (set `PlayerController.bShowMouseCursor` false (`GameplayStatics.GetPlayerController` 0))
      (set `self.GameStates` "NewEnumerator1")
      (bind _returnvalue (`|CreateWidget` "/Game/Widgets/W_InGame.W_InGame_C"))
      (bind _output_get (set `self.InGameWidget` _returnvalue))
      (`UserWidget.AddToPlayerScreen` _output_get 0)
      (`/Game/Widgets/W_InGame.ChangeObjective` _output_get (`/Game/Blueprint/ObjectiveSystem/Objective.Text` (`|GetArrayItem` (`self._Objective`))))
      (`self.OpenLevelText` (`KismetTextLibrary.Conv_StringToText` (`.IntroText_21_E555E9FD4E45C804F745DAB3CD102883` (break `/Game/Blueprint/Managers/LevelInfo` (`self.LevelInfo`))))))
    (:`CastFailed`
      (`KismetSystemLibrary.PrintString` "Instance Cast Failed"))))

(event `self.SpawnPlayerBP`
  (bind _player (`self.Player`))
  ;[1 1 1] Player Spawn Override
  (bind _transform (`self.ZoneChange` 1))
  (bind _returnvalue (`|SpawnActorFromClass` "/Game/Blueprint/P_PlayerPawn.P_PlayerPawn_C" _transform "Undefined" "OverrideRootScale" null "100.000000,100.000000,100.000000|-0.000014,-179.999969,-179.999969|1.000000,1.000000,1.000000" null))
  (bind _output_get (set `/Game/Blueprint/Controller/C_PlayerController.OwnedPawn` _returnvalue _player))
  (`/Game/Blueprint/Controller/C_PlayerController.Init` _player)
  (`/Game/Blueprint/P_PlayerPawn.Init` _output_get)
  (`Controller.Possess` _player _output_get)
  (set `/Game/Blueprint/Controller/C_PlayerController.CurrentPoint` 1 _player))

(fn `GetTarget`
  (locals (Targets :type "Array of /Game/Blueprint/Target Object Reference")))

(fn `UserConstructionScript`)