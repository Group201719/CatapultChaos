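; Tutorial game mode that runs the level from the pregame menu through objectives to the win or end screen.
; On BeginPlay it gathers managers and objectives through interfaces, binds objective completion, then spawns and possesses the player pawn at the first objective's transform.
; StartGame swaps to the in-game HUD, and EndGame fires once all objectives complete.
; DepthTargets toggles target lighting through TargetManagers, while the taunt messages are left unwired.
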(event `CustomEvent`
  (`self.SpawnPlayerBP`))

(event `CustomEvent_1`
  (`self.SetupManagersBP`))

(event `CustomEvent_2`
  (bind _outactors (`self.SetupObjectivesBP`))
  (set `self._Objective` _outactors))

(event `self.CheckObjectives`
  (bind _complete (`self.AreObjectivesCompleteBP`))
  (if _complete
    (`self.EndGame` true)))

(event `ObjectiveComplete`
  (params (Objective :type "/Game/ObjectiveSystem/Objective Object Reference") (Complete :type Boolean))
  ;[1 1 1] Track Objectives and completions
  (bind _complete (`self.AreObjectivesCompleteBP`))
  (if _complete
    (`self.EndGame` true)))

(event `self.ReceiveBeginPlay`
  (`self.Init`))

(event `Init`
  (bind _asc_tutorial_controller (cast `/Game/Base/Controller/C_TutorialController` (`GameplayStatics.GetPlayerController` 0)))
  (set `self.Player` _asc_tutorial_controller)
  (bind _returnvalue (`|CreateWidget` "/Game/Widgets/W_Pregame.W_Pregame_C"))
  (`UserWidget.AddToPlayerScreen` _returnvalue 0)
  (`WidgetBlueprintLibrary.SetInputMode_GameAndUIEx` (`self.Player`) (`/Game/Widgets/W_Pregame.B_StartGame` _returnvalue))
  (bind _controllerwidget (`/Game/Widgets/W_Pregame.SpawnControllerWidget` _returnvalue))
  (set `/Game/Base/Controller/C_TutorialController.TutorialWidget` _controllerwidget (`self.Player`))
  (set `self.GameStates` "NewEnumerator0")
  (`self.SetupManagersBP`)
  (bind _outactors (`self.SetupObjectivesBP`))
  (bind _output_get (set `self._Objective` _outactors))
  (for _array_element _output_get
    ;[1 1 1] Track Objectives and completions
    (`/Game/ObjectiveSystem/Objective.Init` _array_element (`/Game/ObjectiveSystem/Objective.Type` _array_element))
    (add `/Game/ObjectiveSystem/Objective.ObjectiveComplete` _array_element (delegate `ObjectiveComplete`)))
  (`self.SpawnPlayerBP`) ; SpawnPlayer
)

(event `self.StartGame`
  ;[1 1 1] Start Game
  (`WidgetLayoutLibrary.RemoveAllWidgets`)
  (set `PlayerController.bShowMouseCursor` false (`GameplayStatics.GetPlayerController` 0))
  (set `self.GameStates` "NewEnumerator1")
  (bind _returnvalue (`|CreateWidget` "/Game/Widgets/W_InGame.W_InGame_C"))
  (bind _output_get (set `self.InGameWidget` _returnvalue))
  (`UserWidget.AddToPlayerScreen` _output_get 0)
  (`/Game/Widgets/W_InGame.ChangeObjective` _output_get (`/Game/ObjectiveSystem/Objective.Text` (`|GetArrayItem` (`self._Objective`)))))

(event `self.EndGame`
  (params (Win :type Boolean))
  ;[1 1 1] End The game
  (if (and Win (`|EnumEquality` (`self.GameStates`) "NewEnumerator1"))
    (`WidgetLayoutLibrary.RemoveAllWidgets`)
    (bind _returnvalue (`|CreateWidget` "/Game/Widgets/W_WinGame.W_WinGame_C"))
    (`UserWidget.AddToPlayerScreen` _returnvalue 0)
    (else
      (`WidgetLayoutLibrary.RemoveAllWidgets`)
      (bind _returnvalue_2 (`|CreateWidget` "/Game/Widgets/W_Endgame.W_Endgame_C"))
      (`UserWidget.AddToPlayerScreen` _returnvalue_2 0))))

(event `self.DepthTargets`
  (params (Hidden :type Boolean))
  ;[1 1 1] Shit code 101 - change if it works
  (bind _filteredarray (`KismetArrayLibrary.FilterArray` (`self.ActiveManagers`) "/Game/Managers/TargetManager.TargetManager_C"))
  (for _array_element _filteredarray
    (bind _astarget_manager (cast `/Game/Managers/TargetManager` _array_element))
    (`/Game/Managers/TargetManager.LightTargets` _astarget_manager Hidden)))

(event `UpdateTaunt`
  (params (Taunt :type "Actor Class Reference"))
  ;[1 1 1] Taunt System
  (`self.Taunt` Taunt (`self.InGameWidget`)))

(fn `AreObjectivesCompleteBP`
  (returns (Complete :type Boolean))
  (locals (Completes :type "Array of Boolean"))
  (bind __objective (`self._Objective`))
  (for _array_element __objective
    (if (`/Game/ObjectiveSystem/Objective.Complete` _array_element)
      (`KismetArrayLibrary.Array_Add` (`local.Completes`) true)))
  (if (== (`KismetArrayLibrary.Array_Length` __objective) (`KismetArrayLibrary.Array_Length` (`local.Completes`)))
    (return true)
    (else
      (return false))))

(fn `GetGameState`
  (returns (GameState :type "/Game/E_GameStates Enum"))
  (return (`self.GameStates`)))

(fn `GetObjectives`
  (returns (Objectives :type "Array of /Game/ObjectiveSystem/Objective Object Reference"))
  (return (`self._Objective`)))

(fn `SetupManagersBP`
  (returns (ActiveManagers :type "Array of /Game/Base/BaseManager Object Reference"))
  (locals (Tempmanagers :type "Array of /Game/Base/BaseManager Object Reference"))
  (bind _outactors (`GameplayStatics.GetAllActorsWithInterface` "/Game/Interfaces/I_Managers.I_Managers_C"))
  (for _array_element _outactors
    (message `/Game/Interfaces/I_Managers.Init` _array_element)
    (bind _asbase_manager (cast `/Game/Base/BaseManager` _array_element))
    (`KismetArrayLibrary.Array_Add` (`local.Tempmanagers`) _asbase_manager))
  (bind _output_get (set `self.ActiveManagers` (`local.Tempmanagers`)))
  (return _output_get))

(fn `SetupObjectivesBP`
  (returns (OutActors :type "Array of /Game/ObjectiveSystem/Objective Object Reference"))
  (locals (Objectives :type "Array of /Game/ObjectiveSystem/Objective Object Reference"))
  (bind _outactors (`GameplayStatics.GetAllActorsWithInterface` "/Game/ObjectiveSystem/IObjective.IObjective_C"))
  (for _array_element _outactors
    (bind _asobjective (cast `/Game/ObjectiveSystem/Objective` _array_element))
    (`KismetArrayLibrary.Array_Add` (`local.Objectives`) _asobjective))
  (return (`local.Objectives`)))

(fn `SpawnPlayerBP`
  (bind _player (`self.Player`))
  (bind _returnvalue (`|SpawnActorFromClass` "/Game/Base/P_PlayerPawn.P_PlayerPawn_C" (`/Game/ObjectiveSystem/Objective.SpawnTransform` (`|GetArrayItem` (`self._Objective`))) "Undefined" "OverrideRootScale" null "100.000000,100.000000,100.000000|-0.000014,-179.999969,-179.999969|1.000000,1.000000,1.000000" null))
  (bind _output_get (set `/Game/Base/Controller/C_PlayerController.OwnedPawn` _returnvalue _player))
  (`/Game/Base/Controller/C_PlayerController.Init` _player)
  (`/Game/Base/P_PlayerPawn.Init` _output_get)
  (`Controller.Possess` _player _output_get)
  (set `/Game/Base/Controller/C_PlayerController.CurrentPoint` 1 _player)
  (`/Game/Base/Controller/C_PlayerController.LoadSpecificShot` _player "/Game/Base/Projectiles/A_Chicken.A_Chicken_C")
  (return))

(fn `Taunt`
  (params (ProjectileName :type "Actor Class Reference") (Widget :type "/Game/Widgets/W_InGame Object Reference"))
  (switch `string` (`KismetSystemLibrary.GetClassDisplayName` ProjectileName)))

(fn `UserConstructionScript`)